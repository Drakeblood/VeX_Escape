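; BP_CoinsTrack is a placeable actor that lays out a row of child actors, presumably coins, along a spline.
; Its construction script adds CoinAmount child actor components at even distances from the spline's start to its end.
; Each world-space spline location is converted to actor-local space, while the world-space rotation is applied directly as relative rotation.
; The spacing divides by CoinAmount minus one, so a single coin divides by zero.
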(fn ConstructionScript
  (bind _coinamount (Variables|Default|GetCoinAmount))
  (bind _returnvalue (- _coinamount 1))
  (if (> _coinamount 0)
    (for _index (range 0 _returnvalue)
      (AddComponent|AddChildActorComponent false (Math|Transform|MakeTransform (Math|Transform|InverseTransformLocation (Transformation|GetActorTransform) (Spline|GetLocationatDistanceAlongSpline (Variables|Default|GetSpline) (* _index (/ (Spline|GetSplineLength (Variables|Default|GetSpline)) (Math|Conversions|ToFloat(Integer) _returnvalue))) "World")) (Spline|GetRotationatDistanceAlongSpline (Variables|Default|GetSpline) (* _index (/ (Spline|GetSplineLength (Variables|Default|GetSpline)) (Math|Conversions|ToFloat(Integer) _returnvalue))) "World") "1.000000,1.000000,1.000000")))))