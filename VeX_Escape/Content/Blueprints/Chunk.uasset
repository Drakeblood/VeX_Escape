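; Chunk is a level segment that reports the BP_Pawn's passage to the ChunkManager.
; Entering its Box adds the chunk's Order to the manager's Order, and touching DisplacementTrigget calls the manager's Displacement.
; The construction script fits that trigger to the Box's +X face, matching its Y and Z extents.
; Random Rock child-actor spawning inside the Box is present but unconnected.
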(event OnComponentBeginOverlap(DisplacementTrigget)
  (params (OverlappedComponent :type Primitive%20Component%20Object%20Reference) (OtherActor :type Actor%20Object%20Reference) (OtherComp :type Primitive%20Component%20Object%20Reference) (OtherBodyIndex :type Integer) (bFromSweep :type Boolean) (SweepResult :type Hit%20Result%20Structure%20%28by%20ref%29))
  (Utilities|Casting|CastToBP_Pawn OtherActor)
  (bind _returnvalue (Actor|GetActorOfClass "/Game/Blueprints/ChunkManager.ChunkManager_C"))
  (Default|Displacement _returnvalue))

(event OnComponentBeginOverlap(Box)
  (params (OverlappedComponent :type Primitive%20Component%20Object%20Reference) (OtherActor :type Actor%20Object%20Reference) (OtherComp :type Primitive%20Component%20Object%20Reference) (OtherBodyIndex :type Integer) (bFromSweep :type Boolean) (SweepResult :type Hit%20Result%20Structure%20%28by%20ref%29))
  (Utilities|Casting|CastToBP_Pawn OtherActor)
  (bind _returnvalue (Actor|GetActorOfClass "/Game/Blueprints/ChunkManager.ChunkManager_C"))
  (Variables|/Game/Blueprints/ChunkManager.ChunkManager_C|SetOrder _returnvalue (+ (Variables|/Game/Blueprints/ChunkManager.ChunkManager_C|GetOrder _returnvalue) (Variables|Default|GetOrder))))

(event EventBeginPlay)

(fn ConstructionScript
  (bind _box (Variables|Default|GetBox))
  (bind _boxextent (Variables|/Script/Engine.BoxComponent|GetBoxExtent _box))
  (Transformation|SetRelativeLocation (Variables|Default|GetDisplacementTrigget) (Math|Vector|MakeVector (.x (Variables|/Script/Engine.BoxComponent|GetBoxExtent (Variables|Default|GetBox))) 0.0 0.0) false false)
  (Components|Box|SetBoxExtent (Variables|Default|GetDisplacementTrigget) (Math|Vector|MakeVector 0.0 (.y _boxextent) (.z _boxextent)) true))