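; BP_Meteorities is a procedural meteor field that scatters randomly scaled rock meshes and gives them spin.
; The construction script derives the rock count from Extent's length divided by Density, so higher Density means fewer rocks, and stores each component in RockArray.
; Random offsets are multiplied by loop index, so potential spread grows with each rock, independent of Extent.
; BeginPlay applies one random torque to each stored rock.
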(event EventBeginPlay
  (for _array_element (Variables|Default|GetRockArray)
    (Class|PrimitiveComponent|AddTorqueinRadians _array_element (Math|Vector|MakeVector (Math|Random|RandomFloatinRange -4e+01 4e+01) (Math|Random|RandomFloatinRange -3e+01 3e+01) (Math|Random|RandomFloatinRange -2e+01 2e+01)) "None" false)))

(event Collision|EventActorBeginOverlap
  (params (OtherActor :type Actor%20Object%20Reference)))

(event EventTick
  (params (DeltaSeconds :type Float%20%28single-precision%29)))

(fn ConstructionScript
  (bind _maxscale (Variables|Default|GetMaxScale))
  (bind _extent (Variables|Default|GetExtent))
  (bind _density (Variables|Default|GetDensity))
  (bind _returnvalue (Math|Random|RandomFloatinRange 0.9 _maxscale))
  (bind _returnvalue_2 (* _extent "1.000000,1.000000,1.000000"))
  (bind _returnvalue_3 (Math|Vector|VectorLength _returnvalue_2))
  (bind _returnvalue_4 (/ _returnvalue_3 _density))
  (bind _returnvalue_5 (Math|Float|Round _returnvalue_4))
  (if (> _returnvalue_5 0)
    (for _index (range 1 _returnvalue_5)
      (bind _returnvalue_6 (AddComponent|AddStaticMeshComponent false (Math|Transform|MakeTransform (Math|Vector|MakeVector (* _index (Math|Random|RandomFloatinRange -1e+03 1e+03)) (* _index (Math|Random|RandomFloatinRange -1e+03 1e+03)) (* _index (Math|Random|RandomFloatinRange -1e+03 1e+03))) "0, 0, 0" (Math|Vector|MakeVector _returnvalue _returnvalue _returnvalue))))
      (Utilities|Array|Add (Variables|Default|GetRockArray) _returnvalue_6))))