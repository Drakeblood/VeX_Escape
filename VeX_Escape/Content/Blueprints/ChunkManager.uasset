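; ChunkManager builds and extends a tiled world of Chunk actors on a fixed-size grid.
; BeginPlay spawns a starting three-by-three block and stores each actor in the Chunks array.
; Displacement spawns another row of three further along X, using the sign of Order to keep it centered or shift it sideways along Y.
; Running X, left and right offsets track the next row's position; nothing here removes old chunks.
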(event EventBeginPlay
  (for _index (range 0 2)
    (for _index_2 (range 0 2)
      (switch int _index
        (:0
          (bind _returnvalue (Game|SpawnActorfromClass "/Game/Blueprints/Chunk.Chunk_C" (Math|Conversions|ToTransform(Vector) (Math|Vector|MakeVector 0.0 (+ -8e+03 (* _index_2 8e+03)) 0.0)) "Undefined" 0 0))
          (Utilities|Array|Add (Variables|Default|GetChunks) _returnvalue))
        (:1
          (bind _returnvalue_2 (Game|SpawnActorfromClass "/Game/Blueprints/Chunk.Chunk_C" (Math|Conversions|ToTransform(Vector) (Math|Vector|MakeVector 8e+03 (+ -8e+03 (* _index_2 8e+03)) 0.0)) "Undefined" 0 0))
          (Utilities|Array|Add (Variables|Default|GetChunks) _returnvalue_2))
        (:2
          (bind _returnvalue_3 (Game|SpawnActorfromClass "/Game/Blueprints/Chunk.Chunk_C" (Math|Conversions|ToTransform(Vector) (Math|Vector|MakeVector 1.6e+04 (+ -8e+03 (* _index_2 8e+03)) 0.0)) "Undefined" 0 0))
          (Utilities|Array|Add (Variables|Default|GetChunks) _returnvalue_3))))))

(fn ConstructionScript)

(fn Displacement
  (if (== (Variables|Default|GetOrder) 0)
    (for _index (range 0 2)
      (bind _returnvalue (Game|SpawnActorfromClass "/Game/Blueprints/Chunk.Chunk_C" (Math|Conversions|ToTransform(Vector) (Math|Vector|MakeVector (Variables|Default|GetCurrentXReplacement) (+ (- (Variables|Default|GetCurrentRightReplacement) 8e+03) (* _index 8e+03)) 0.0)) "Undefined" 0 0))
      (Utilities|Array|Add (Variables|Default|GetChunks) _returnvalue))
    (Variables|Default|SetCurrentXReplacement (+ (Variables|Default|GetCurrentXReplacement) 8e+03))
    (elif (< (Variables|Default|GetOrder) 0)
      (for _index_2 (range 0 2)
        (bind _returnvalue_2 (Game|SpawnActorfromClass "/Game/Blueprints/Chunk.Chunk_C" (Math|Conversions|ToTransform(Vector) (Math|Vector|MakeVector (Variables|Default|GetCurrentXReplacement) (+ (Variables|Default|GetCurrentLeftReplacement) (* _index_2 8e+03)) 0.0)) "Undefined" 0 0))
        (Utilities|Array|Add (Variables|Default|GetChunks) _returnvalue_2))
      (Variables|Default|SetCurrentLeftReplacement (+ (Variables|Default|GetCurrentLeftReplacement) -8e+03))
      (Variables|Default|SetCurrentXReplacement (+ (Variables|Default|GetCurrentXReplacement) 8e+03))
      (Variables|Default|SetCurrentRightReplacement (+ (Variables|Default|GetCurrentRightReplacement) -8e+03))
      (elif (> (Variables|Default|GetOrder) 0)
        (for _index_3 (range 0 2)
          (bind _returnvalue_3 (Game|SpawnActorfromClass "/Game/Blueprints/Chunk.Chunk_C" (Math|Conversions|ToTransform(Vector) (Math|Vector|MakeVector (Variables|Default|GetCurrentXReplacement) (+ (Variables|Default|GetCurrentRightReplacement) (* _index_3 8e+03)) 0.0)) "Undefined" 0 0))
          (Utilities|Array|Add (Variables|Default|GetChunks) _returnvalue_3))
        (Variables|Default|SetCurrentRightReplacement (+ (Variables|Default|GetCurrentRightReplacement) 8e+03))
        (Variables|Default|SetCurrentXReplacement (+ (Variables|Default|GetCurrentXReplacement) 8e+03))
        (Variables|Default|SetCurrentLeftReplacement (+ (Variables|Default|GetCurrentLeftReplacement) 8e+03))))))