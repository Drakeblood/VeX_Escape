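; Asteroid belt actor that scatters randomized asteroid meshes along a spline.
; The construction script adds individual static mesh components at even intervals along the spline, each with a large random positional offset, random rotation and random uniform scale times ScaleMultiplier.
; AsteroidAmount sets the density, and each component is stored in MeteoritesArray.
; BeginPlay applies a one-time random torque to each stored mesh to start it tumbling.
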(event EventBeginPlay
  (for _array_element (Variables|Default|GetMeteoritesArray)
    (Class|PrimitiveComponent|AddTorqueinRadians _array_element (Math|Vector|MakeVector (Math|Random|RandomFloatinRange -3e+01 3e+01) (Math|Random|RandomFloatinRange -2e+01 2e+01) (Math|Random|RandomFloatinRange -1e+01 5.0)) "None" false)))

(fn ConstructionScript
  (bind _returnvalue (Math|Random|RandomFloatinRange -1.8e+02 1.8e+02))
  (bind _asteroidamount (Variables|Default|GetAsteroidAmount))
  (if (> _asteroidamount 0)
    (for _index (range 0 _asteroidamount)
      (bind _returnvalue_2 (AddComponent|AddStaticMeshComponent false (Math|Transform|MakeTransform (Math|Vector|MakeVector (+ (.X (Math|Vector|BreakVector (Math|Transform|InverseTransformLocation (Transformation|GetActorTransform) (Spline|GetLocationatDistanceAlongSpline (Variables|Default|GetSpline) (* _index (/ (Spline|GetSplineLength (Variables|Default|GetSpline)) (Math|Conversions|ToFloat(Integer) _asteroidamount))) "World")))) (Math|Random|RandomFloatinRange -1e+05 1e+05)) (+ (.Y (Math|Vector|BreakVector (Math|Transform|InverseTransformLocation (Transformation|GetActorTransform) (Spline|GetLocationatDistanceAlongSpline (Variables|Default|GetSpline) (* _index (/ (Spline|GetSplineLength (Variables|Default|GetSpline)) (Math|Conversions|ToFloat(Integer) _asteroidamount))) "World")))) (Math|Random|RandomFloatinRange -1e+05 1e+05)) (+ (.Z (Math|Vector|BreakVector (Math|Transform|InverseTransformLocation (Transformation|GetActorTransform) (Spline|GetLocationatDistanceAlongSpline (Variables|Default|GetSpline) (* _index (/ (Spline|GetSplineLength (Variables|Default|GetSpline)) (Math|Conversions|ToFloat(Integer) _asteroidamount))) "World")))) (Math|Random|RandomFloatinRange -1e+05 1e+05))) (Math|Rotator|MakeRotator _returnvalue _returnvalue _returnvalue) (Math|Conversions|ToVector(Float) (* (Math|Random|RandomFloatinRange 0.7 2e+01) (Variables|Default|GetScaleMultiplier))))))
      (Utilities|Array|Add (Variables|Default|GetMeteoritesArray) _returnvalue_2))))