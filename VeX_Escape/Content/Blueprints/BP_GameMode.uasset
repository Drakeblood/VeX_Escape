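; Game mode that reports when the player pawn strays beyond a sector's extent, using its VEX sector manager component.
; On BeginPlay it binds to the component's displacement event, which compares the pawn with the first wall's center on Y and Z independently.
; Exceeding the extent only prints Right/Left or Up/Down, judged by the direction's sign.
; A separate VEPrint event and unwired distance/direction prints serve as debug output.
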(event Custom|VEPrint
  (Development|PrintString (Utilities|String|ToString(Vector) (Variables|Default|GetVE))))

(event Custom|OnDisplacementEvent
  (bind _returnvalue (Game|Player|GetPlayerPawn 0))
  (bind _vexsectormanagercomponent (Variables|Default|GetVEXSectorManagerComponent))
  (bind _vexsectormanagercomponent_2 (Variables|Default|GetVEXSectorManagerComponent))
  (bind _returnvalue_2 (Transformation|GetActorLocation _returnvalue))
  (bind _returnvalue_3 (Class|VEXSectorManagerComponent|GetSectorExtent _vexsectormanagercomponent_2))
  (bind _returnvalue_4 (Transformation|GetActorLocation _returnvalue))
  (bind _walls (Variables|/Script/VeX_Escape.VEXSectorManagerComponent|GetWalls _vexsectormanagercomponent))
  (bind _output (Utilities|Array|Get(acopy) _walls))
  (bind _returnvalue_5 (Class|VEXWallBase|GetCenterLocation _output))
  (bind _returnvalue_6 (Class|VEXWallBase|GetCenterLocation _output))
  (bind _returnvalue_7 (Math|Vector|GetUnitDirection(Vector) _returnvalue_6 _returnvalue_2))
  (bind (_x _y _z) (Math|Vector|BreakVector _returnvalue_7))
  (Utilities|IsValid _output
    (:Is%20Valid
      (if (> (Math|Vector|Distance(Vector) (Math|Vector|MakeVector 0.0 (.y _returnvalue_5) 0.0) (Math|Vector|MakeVector 0.0 (.y _returnvalue_4) 0.0)) (.y _returnvalue_3))
        (Utilities|FlowControl|Sequence
          (:then_0
            (if (> _y 0.0)
              (Development|PrintString "Right")))
          (:then_1
            (if (< _y 0.0)
              (Development|PrintString "Left")))
          (:then_2
            (if (> (Math|Vector|Distance(Vector) (Math|Vector|MakeVector 0.0 0.0 (.z _returnvalue_5)) (Math|Vector|MakeVector 0.0 0.0 (.z _returnvalue_4))) (.z _returnvalue_3)) :!label _label
              (Utilities|FlowControl|Sequence
                (:then_0
                  (if (> _z 0.0)
                    (Development|PrintString "Up")))
                (:then_1
                  (if (< _z 0.0)
                    (Development|PrintString "Down")))))))
        (else
          (goto _label))))))

(event EventBeginPlay
  (|CallParentFunction)
  (EventDispatchers|AssignOnDisplacement (Variables|Default|GetVEXSectorManagerComponent) (delegate Custom|OnDisplacementEvent)))

(fn ConstructionScript)