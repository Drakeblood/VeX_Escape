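; BP_Sector is a box-bounded region of space that fills itself with drifting, tumbling rocks.
; On BeginPlay it spawns five BP_Rock actors at random points in SectorBox with random rotation and scale, attaches them and applies random torque and force.
; When the displacement event fires, it recycles the same rocks rather than respawning, scattering them to new points in the box and applying fresh random impulse-like pushes.
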(event EventBeginPlay
  (bind _sectorbox (Variables|Default|GetSectorBox))
  (for _index (range 1 5)
    (bind _returnvalue (Game|SpawnActorfromClass "/Game/Blueprints/Gameplay/Obstacles/BP_Rock.BP_Rock_C" (Math|Transform|MakeTransform (Math|Random|RandomPointinBoundingBox (Transformation|GetWorldLocation _sectorbox) (Variables|/Script/Engine.BoxComponent|GetBoxExtent _sectorbox)) (Math|Random|RandomRotator false) (CallFunction|GetRandomVectorinRange 1.0 5.0)) "Undefined" 0 0))
    (Transformation|AttachActorToActor _returnvalue self "None" "KeepWorld" "KeepRelative" "KeepRelative" true)
    (Class|PrimitiveComponent|AddTorqueinRadians (Variables|/Game/Blueprints/Gameplay/Obstacles/BP_Rock.BP_Rock_C|GetRockStaticMesh _returnvalue) (CallFunction|GetRandomVectorinRange -4e+02 4e+02) "None" false)
    (Utilities|Array|Add (Variables|Default|GetRocks) _returnvalue)
    (Physics|AddForce (Variables|/Game/Blueprints/Gameplay/Obstacles/BP_Rock.BP_Rock_C|GetRockStaticMesh _returnvalue) (CallFunction|GetRandomVectorinRange -2e+01 2e+01) "None" false)))

(event EventOnDisplacementBlueprintEvent
  (bind _sectorbox (Variables|Default|GetSectorBox))
  (for _array_element (Variables|Default|GetRocks)
    (Transformation|SetActorLocation _array_element (Math|Random|RandomPointinBoundingBox (Transformation|GetWorldLocation _sectorbox) (Variables|/Script/Engine.BoxComponent|GetBoxExtent _sectorbox)) false false)
    (Class|PrimitiveComponent|AddTorqueinRadians (Variables|/Game/Blueprints/Gameplay/Obstacles/BP_Rock.BP_Rock_C|GetRockStaticMesh _array_element) (Math|Vector|MakeVector (Math|Random|RandomFloatinRange -4e+02 4e+02) (Math|Random|RandomFloatinRange -4e+02 4e+02) (Math|Random|RandomFloatinRange -4e+02 4e+02)) "None" false)
    (Physics|AddForce (Variables|/Game/Blueprints/Gameplay/Obstacles/BP_Rock.BP_Rock_C|GetRockStaticMesh _array_element) (Math|Conversions|ToVector(Float) (Math|Random|RandomFloatinRange -2e+01 2e+01)) "None" false)))

(fn ConstructionScript)