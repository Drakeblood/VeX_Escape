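; BP_StartField is an actor that procedurally builds a star field from instanced meshes in its construction script.
; It adds StarCount-driven instances to the Star component at random positions within configurable XYZ extents, with random per-axis scale.
; Each loop pass creates a dynamic M_Star material, using the instance index as the material element index, and sets color and fade parameters.
; The event graph is empty.
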(event EventBeginPlay)

(event Collision|EventActorBeginOverlap
  (params (OtherActor :type Actor%20Object%20Reference)))

(event EventTick
  (params (DeltaSeconds :type Float%20%28single-precision%29)))

(fn ConstructionScript
  (bind _starfieldx (Variables|Default|GetStarFieldX))
  (bind _starfieldz (Variables|Default|GetStarFieldZ))
  (bind _starminscale (Variables|Default|GetStarMinScale))
  (bind _starmaxscale (Variables|Default|GetStarMaxScale))
  (bind _starfieldy (Variables|Default|GetStarFieldY))
  (bind _returnvalue (Math|Random|RandomFloatinRange _starminscale _starmaxscale))
  (for _index (range 0 (Variables|Default|GetStarCount))
    (bind _returnvalue_2 (Components|InstancedStaticMesh|AddInstance (Variables|Default|GetStar) (Math|Transform|MakeTransform (Math|Vector|MakeVector (Math|Random|RandomFloatinRange (* _starfieldx -1.0) _starfieldx) (Math|Random|RandomFloatinRange (* _starfieldy -1.0) _starfieldy) (Math|Random|RandomFloatinRange (* _starfieldz -1.0) _starfieldz)) "0, 0, 0" (Math|Vector|MakeVector _returnvalue _returnvalue _returnvalue))))
    (bind _returnvalue_3 (Rendering|Material|CreateDynamicMaterialInstance (Variables|Default|GetStar) _returnvalue_2 "/Game/M_Star.M_Star" "None" :!class /Script/Engine.PrimitiveComponent))
    (Rendering|Material|SetVectorParameterValue _returnvalue_3 "Color 1" (Variables|Default|GetColor%201) :!class /Script/Engine.MaterialInstanceDynamic)
    (Rendering|Material|SetVectorParameterValue _returnvalue_3 "Color 2" (Variables|Default|GetColor%202) :!class /Script/Engine.MaterialInstanceDynamic)
    (Rendering|Material|SetScalarParameterValue _returnvalue_3 "StarColorDistance" (Variables|Default|GetStarColorDistance) :!class /Script/Engine.MaterialInstanceDynamic)
    (Rendering|Material|SetScalarParameterValue _returnvalue_3 "StarColorFade" (Variables|Default|GetStarColorFade) :!class /Script/Engine.MaterialInstanceDynamic)))